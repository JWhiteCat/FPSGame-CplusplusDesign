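; BP_TestGameMode is a test game mode holding wave spawning, kill scoring and main menu logic, all currently disconnected.
; An EQS finished handler draws debug spheres and spawns BP_TrackeBot at each resulting location.
; A kill handler adds score to the killer pawn's SPlayerState and prints it.
; BeginPlay is empty, so the query launch, kill-delegate binding and WBP_MainMenu creation never run.
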(event `OnQueryFinishedEvent_Event_0`
  (params (QueryInstance :type "EnvQueryInstanceBlueprintWrapper Object Reference") (QueryStatus :type "EEnvQueryStatus Enum" :default "Processing"))
  ;[1 1 1] Wave
  (switch `EEnvQueryStatus` QueryStatus
    (:`Success`
      (for _array_element (`EnvQueryInstanceBlueprintWrapper.GetResultsAsLocations` QueryInstance)
        (`KismetSystemLibrary.DrawDebugSphere` _array_element 50.0 12 (struct :`R` 0.919079 :`G` 1.0 :`A` 1.0) 2.0 2.0)
        (`|SpawnActorFromClass` "/Game/BluePrints/BP_TrackeBot.BP_TrackeBot_C" (`KismetMathLibrary.MakeTransform` _array_element) "AdjustIfPossibleButDontSpawnIfColliding" "OverrideRootScale" null null)))))

(event `self.ReceiveBeginPlay`)

(event `OnActorKilled_Event_0` :!signature `self.OnActorKilled`
  (params (VictimActor :type "Actor Object Reference") (KillerActor :type "Actor Object Reference") (KillerController :type "Controller Object Reference"))
  (bind _assplayer_state (cast `SPlayerState` (`Pawn.PlayerState` (`Controller.K2_GetPawn` KillerController))))
  (`SPlayerState.AddScore` _assplayer_state 20.0)
  (`KismetSystemLibrary.PrintString` (`KismetStringLibrary.Conv_DoubleToString` (`PlayerState.Score` _assplayer_state))))

(fn `UserConstructionScript`)