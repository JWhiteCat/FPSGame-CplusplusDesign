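; Game mode Blueprint that opens the main menu and runs kill-based scoring with a win announcement.
; On BeginPlay it shows the mouse cursor, adds WBP_MainMenu to the viewport and binds to the OnActorKilled delegate.
; Each kill casts the killer controller's pawn to PlayerPawn, adds points to its SPlayerState and prints a winner message once the score reaches the threshold.
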(event `self.ReceiveBeginPlay`
  (`|ExecutionSequence`
    (:`then_0`
      (set `PlayerController.bShowMouseCursor` true (`GameplayStatics.GetPlayerController` 0))
      (bind _returnvalue (`|CreateWidget` "/Game/UI/WBP_MainMenu.WBP_MainMenu_C"))
      (`UserWidget.AddToViewport` _returnvalue 0))
    (:`then_1`
      (add `self.OnActorKilled` (delegate `OnActorKilled_Event_0`)))))

(event `OnActorKilled_Event_0` :!signature `self.OnActorKilled`
  (params (VictimActor :type "Actor Object Reference") (KillerActor :type "Actor Object Reference") (KillerController :type "Controller Object Reference"))
  (bind _asplayer_pawn (cast `/Game/BluePrints/PlayerPawn` (`Controller.K2_GetPawn` KillerController)))
  (bind _playerstate (`Pawn.PlayerState` _asplayer_pawn))
  (bind _assplayer_state (cast `SPlayerState` _playerstate))
  (`SPlayerState.AddScore` _assplayer_state 20.0)
  (if (>= (`PlayerState.Score` _assplayer_state) 40.0)
    (`KismetSystemLibrary.PrintString` (`KismetTextLibrary.Conv_TextToString` (`|FormatText` "Player{ID} 获胜!!" (`PlayerState.PlayerId` _playerstate))))))

(fn `UserConstructionScript`)